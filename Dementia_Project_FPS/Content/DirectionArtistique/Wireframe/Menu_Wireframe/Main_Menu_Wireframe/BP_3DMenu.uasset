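; BP_3DMenu is a wireframe main-menu actor that hosts a 3DMain_Widget and links to other menus.
; On BeginPlay it binds to the widget's transition event and disables its own collision.
; The event's menu index selects a target from the LinkedMenu array.
; The transition then disables collision here, enables it on the target and eases the player's view to that menu over a timed camera blend.
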(event `self.ReceiveBeginPlay`
  ;[1 1 1] Permet de faire la transition entre les différents menus selon quel ``Menu Index`` est appelé
  (bind _as3dmain_widget (cast `/Game/DirectionArtistique/Wireframe/Menu_Wireframe/Main_Menu_Wireframe/3DMain_Widget` (`WidgetComponent.GetUserWidgetObject` (`self.Widget`))))
  (add `/Game/DirectionArtistique/Wireframe/Menu_Wireframe/Main_Menu_Wireframe/3DMain_Widget.TransitionToLinkedMap` _as3dmain_widget (delegate `OnTransitionBetweenMenu`))
  (`self.SetActorEnableCollision` false))

(event `OnTransitionBetweenMenu`
  (params (MenuIndex :type Integer))
  ;[1 1 1] Permet de faire la transition entre les différents menus selon quel ``Menu Index`` est appelé
  (if (`KismetArrayLibrary.Array_IsValidIndex` (`self.LinkedMenu`) MenuIndex)
    (`self.TransitionToCamera` (`|GetArrayItem` (`self.LinkedMenu`) MenuIndex))))

(event `TransitionToCamera`
  (params (NewMenu :type "/Game/DirectionArtistique/Wireframe/Menu_Wireframe/Main_Menu_Wireframe/BP_3DMenu Object Reference"))
  ;[1 1 1] Permet au joueur changer de menu et de se fixer sur la camera de ce menu
  (`self.SetActorEnableCollision` false)
  (`self.SetActorEnableCollision` NewMenu true)
  (`PlayerController.SetViewTargetWithBlend` (`GameplayStatics.GetPlayerController` 0) NewMenu 2.0 "VTBlend_EaseInOut" 2.0 false))

(fn `UserConstructionScript`)