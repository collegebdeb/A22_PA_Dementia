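; BP_Gramophone is a spinning gramophone actor that plays a sound and acts as a level transition trigger.
; On BeginPlay it assigns SoundList to its Audio component, and Tick derives a steady mesh yaw rotation from game time.
; When the first-person character overlaps it, it calls FadeOut through that character's fade reference, waits briefly, then opens the level named by LevelName.
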(event `self.ReceiveBeginPlay`
  (`self.Choose_Musique`))

(event `Choose_Musique`
  (`AudioComponent.SetSound` (`self.Audio`) (`self.Sound_List`)))

(event `self.ReceiveActorBeginOverlap`
  (params (OtherActor :type "Actor Object Reference"))
  (bind _asbp_first_person_character (cast `/Game/FirstPerson/Blueprints/BP_FirstPersonCharacter` OtherActor))
  (`/Game/Wireframe/Fade_Widget.Fade_Out` (`/Game/FirstPerson/Blueprints/BP_FirstPersonCharacter.Fade_Ref` _asbp_first_person_character))
  (`KismetSystemLibrary.Delay` 1.0)
  (`GameplayStatics.OpenLevel` (`self.Level Name`)))

(event `self.ReceiveTick`
  (params (DeltaSeconds :type "Float (single-precision)"))
  (`SceneComponent.K2_SetRelativeRotation` (`self.StaticMesh`) (`KismetMathLibrary.MakeRotator` 0.0 0.0 (* (`GameplayStatics.GetTimeSeconds`) 90.0)) false false))

(fn `UserConstructionScript`)